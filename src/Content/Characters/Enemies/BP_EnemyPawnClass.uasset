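; BP_EnemyPawnClass is an enemy pawn that homes in on the player.
; BeginPlay caches the first BP_PlayerCharacterController actor as its Target.
; Each Tick, MoveEnemyTowardsPlayer offsets the pawn along the normalized direction to Target, scaled by EnemySpeed.
; Movement is frame-rate dependent, with no delta-time scaling, and skips collision sweeps.
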(event EventBeginPlay
  ;[1 1 1] Get Player Reference
  (bind _returnvalue (Actor|GetActorOfClass "/Game/Blueprints/Player/BP_PlayerCharacterController.BP_PlayerCharacterController_C"))
  (Variables|Default|SetTarget _returnvalue))

(event EventTick
  (params (DeltaSeconds :type Float%20%28single-precision%29))
  ;[1 1 1] Get Player Reference
  (CallFunction|MoveEnemyTowardsPlayer))

(fn ConstructionScript)

(fn MoveEnemyTowardsPlayer
  (Transformation|AddActorWorldOffset self (* (Math|Vector|Normalize (- (Transformation|GetActorLocation (Variables|Default|GetTarget)) (Transformation|GetActorLocation self))) (Math|Conversions|ToVector(Float) (Variables|Default|GetEnemySpeed))))
  (return))