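; Actor component that plays flipbook sprite animations on a character's static mesh, found by name on the owner at BeginPlay.
; SetAnimationType picks a sprite and looping or one-shot mode; Tick advances frames and fires frame-indexed notifies, such as a Niagara fire burst.
; Frame progress, sprite index, and lerped damage-flash and selection highlights reach the material through Custom Primitive Data.
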(event Custom|SetAnimationType
  (params (SpriteType :type String) (AnimationType :type EAnimationType%20Enum :default "AnimationType_MAX") (AnimationNotifyFrames :type Array%20of%20Integers) (AnimationNotifyNames :type Array%20of%20Strings) (AnimationSpeed :type Float%20%28double-precision%29))
  ;[1 1 1] Used to change the animation, we want to set the flipbook to the first frame every time we call this
  (Variables|AnimationParameters|SetAnimationSpeed AnimationSpeed)
  (Variables|AnimationParameters|SetCurrentAnimationNotifyNames AnimationNotifyNames)
  (Variables|AnimationParameters|SetCurrentAnimationNotifyFrames AnimationNotifyFrames)
  (Variables|AnimationParameters|SetAnimNotifyIndex 0)
  (AnimationFunctions|SelectAnimationType SpriteType AnimationType)
  ;[1 1 1] Set the correlated material values relating to the sprite type
  (MaterialFunctions|SetMaterialCustomPrimitiveData))

(event Custom|SetTypeOfCharacterAnimatorBehaviour
  (params (TypeOfCharacterInput :type String)))

(event Custom|Select
  (params (SelectTarget? :type Boolean))
  ;[1 1 1] Use this to toggle selection of this character so the player knows what they are about to interact with
  (if SelectTarget?
    (Variables|MaterialParameters|SetSelectBool true)
    (Variables|MaterialParameters|SetSelectWeightTarget 1.0)
    (else
      (Variables|MaterialParameters|SetSelectWeightTarget 0.0))))

(event Custom|DamageFlash
  ;[1 1 1] Use this to give a brief flash to indicate the character took damage
  (Variables|MaterialParameters|SetDamageFlashBool true)
  (Variables|MaterialParameters|SetDamageFlashWeightTarget 1.0))

(event Custom|ChangeDamageColor
  (params (NewColor :type Vector))
  ;[1 1 1] Change Damage/Select color of object at runtime if needed
  (Rendering|Material|SetCustomPrimitiveDataVector3 (Variables|Default|GetCharacterStaticMesh) 10 (Math|Vector|MakeVector (.x NewColor) (.y NewColor) (.z NewColor))))

(event Custom|ChangeSelectColor
  (params (NewColor :type Vector))
  ;[1 1 1] Change Damage/Select color of object at runtime if needed
  (Rendering|Material|SetCustomPrimitiveDataVector3 (Variables|Default|GetCharacterStaticMesh) 14 (Math|Vector|MakeVector (.x NewColor) (.y NewColor) (.z NewColor))))

(event Custom|AnimationNotify
  (params (TypeOfAnimationNotify :type String))
  ;[1 1 1] Animation Notifies
  (switch string TypeOfAnimationNotify
    (:SpawnFireParticles
      (Development|PrintString "SpawnFireParticles")
      (EffectsFunctions|SpawnFire))
    (:SpawnFireSound
      (Development|PrintString "SpawnFireSound"))))

(event EventBeginPlay
  ;[1 1 1] Attempt to get the static mesh we want to animate
  (CallFunction|GetStaticMesh))

(event EventTick
  (params (DeltaSeconds :type Float%20%28single-precision%29))
  ;[1 1 1] Tick
  (AnimationFunctions|AnimationTimeIncrement DeltaSeconds)
  (if (or (Variables|MaterialParameters|GetDamageFlashBool) (Variables|MaterialParameters|GetSelectBool))
    (AnimationFunctions|DamageFlashIncrement)
    (AnimationFunctions|SelectTargetIncrement)))

(fn AnimationTimeIncrement
  (params (Time :type Float%20%28double-precision%29))
  ;[1 1 1] Determines what frame to set the flipbook to
  (Variables|AnimationParameters|SetAnimationTime (/ (Math|Conversions|ToFloat(Integer) (Variables|AnimationParameters|GetCurrentFrame)) (Math|Conversions|ToFloat(Integer) (Variables|AnimationParameters|GetCurrentNumberOfFramesInAnimation))))
  (bind _output_get (Variables|AnimationParameters|SetFrameTime (+ (* Time (Variables|AnimationParameters|GetAnimationSpeed)) (Variables|AnimationParameters|GetFrameTime))))
  (if (>= _output_get (Variables|AnimationParameters|GetFrameDuration))
    (if (Variables|AnimationParameters|GetShouldAnimationLoop)
      (bind _output_get_2 (Variables|AnimationParameters|SetCurrentFrame (Math|Integer|%(Integer) (+ (Variables|AnimationParameters|GetCurrentFrame) 1) (Variables|AnimationParameters|GetCurrentNumberOfFramesInAnimation))))
      (Development|PrintString (Utilities|String|ToString(Integer) _output_get_2))
      (else
        (Variables|AnimationParameters|SetCurrentFrame (Math|Integer|Clamp(Integer) (+ (Variables|AnimationParameters|GetCurrentFrame) 1) 0 (Variables|AnimationParameters|GetCurrentNumberOfFramesInAnimation)))))
    (Variables|AnimationParameters|SetFrameTime (- (Variables|AnimationParameters|GetFrameTime) (Variables|AnimationParameters|GetFrameDuration))))
  (Rendering|Material|SetCustomPrimitiveDataFloat (Variables|Default|GetCharacterStaticMesh) 0 (Variables|AnimationParameters|GetAnimationTime))
  ;[1 1 1] Increment or reset index?
  (if (== (Utilities|Array|Get(acopy) (Variables|AnimationParameters|GetCurrentAnimationNotifyFrames) (+ (Variables|AnimationParameters|GetAnimNotifyIndex) 1)) (Variables|AnimationParameters|GetCurrentFrame))
    (if (== (+ (Variables|AnimationParameters|GetAnimNotifyIndex) 1) (Utilities|Array|LastIndex (Variables|AnimationParameters|GetCurrentAnimationNotifyFrames)))
      (Variables|AnimationParameters|SetAnimNotifyIndex 0)
      (else
        (Variables|AnimationParameters|SetAnimNotifyIndex (+ (Variables|AnimationParameters|GetAnimNotifyIndex) 1))
        ;[1 1 1] Call animation notify related to frame index
        (CallFunction|AnimationNotify (Utilities|Array|Get(acopy) (Variables|AnimationParameters|GetCurrentAnimationNotifyNames) (Variables|AnimationParameters|GetAnimNotifyIndex))))))
  (return))

(fn DamageFlashIncrement
  (bind _output_get (Variables|MaterialParameters|SetDamageFlashWeightCurrent (Math|Float|Lerp (Variables|MaterialParameters|GetDamageFlashWeightCurrent) (Variables|MaterialParameters|GetDamageFlashWeightTarget) 0.3)))
  (Rendering|Material|SetCustomPrimitiveDataFloat (Variables|Default|GetCharacterStaticMesh) 4 _output_get)
  (if (> _output_get 0.97)
    (Variables|MaterialParameters|SetDamageFlashWeightTarget 0.0)
    (elif (== (Variables|MaterialParameters|GetDamageFlashWeightCurrent) 0.0)
      (Variables|MaterialParameters|SetDamageFlashBool false)))
  (return))

(fn SelectTargetIncrement
  (bind _output_get (Variables|MaterialParameters|SetCurrentSelectWeight (Math|Float|Lerp (Variables|MaterialParameters|GetCurrentSelectWeight) (Variables|MaterialParameters|GetSelectWeightTarget) 0.1)))
  (Rendering|Material|SetCustomPrimitiveDataFloat (Variables|Default|GetCharacterStaticMesh) 5 _output_get)
  (if (== _output_get 0.0)
    (Variables|MaterialParameters|SetSelectBool false))
  (return))

(fn SelectAnimationType
  (params (InputPin :type String) (Selection :type EAnimationType%20Enum :default "NewEnumerator0"))
  (switch Utilities|FlowControl|Switch|SwitchonEAnimationType Selection
    (:NewEnumerator0
      (Variables|AnimationParameters|SetShouldAnimationLoop true))
    (:NewEnumerator1
      (Variables|AnimationParameters|SetShouldAnimationLoop false)))
  (for (_ _array_index) (Variables|MaterialParameters|GetSprites)
    (if (Utilities|Enum|Equal(Enum) (Utilities|GetObjectName (Utilities|Array|Get(acopy) (Variables|MaterialParameters|GetSprites) _array_index)) InputPin)
      (Variables|MaterialParameters|SetCurrentSpriteIndex _array_index)
      (AnimationFunctions|SetCurrentAnimationNumberOfFrames (Utilities|Array|Get(acopy) (Variables|MaterialParameters|GetRows%20&%20Columns) _array_index))))
  (Variables|AnimationParameters|SetAnimationTime 0.0)
  (Variables|AnimationParameters|SetCurrentFrame 0)
  (return))

(fn SetCurrentAnimationNumberOfFrames
  (params (Rows%20&%20Columns :type Vector%202D%20Structure))
  (Variables|AnimationParameters|SetCurrentNumberOfFramesInAnimation (Math|Float|Truncate (* (.x Rows%20&%20Columns) (.y Rows%20&%20Columns))))
  (return))

(fn SetMaterialCustomPrimitiveData
  (bind _characterstaticmesh (Variables|Default|GetCharacterStaticMesh))
  (Rendering|Material|SetCustomPrimitiveDataFloat _characterstaticmesh 1 (Math|Conversions|ToFloat(Integer) (Variables|MaterialParameters|GetCurrentSpriteIndex)))
  (Rendering|Material|SetCustomPrimitiveDataFloat _characterstaticmesh 2 (Math|Conversions|ToFloat(Integer) (Variables|MaterialParameters|GetCurrentSpriteIndex)))
  (Rendering|Material|SetCustomPrimitiveDataFloat _characterstaticmesh 3 (Math|Conversions|ToFloat(Integer) (Variables|MaterialParameters|GetCurrentSpriteIndex)))
  (return))

(fn SpawnFire
  (Niagara|SpawnSystemAttached "/Niagara/DefaultAssets/Templates/Systems/DirectionalBurst.DirectionalBurst" (Variables|Default|GetCharacterStaticMesh) "None" "0.000000,70.000000,0.000000" "90.000000,-180.000000,90.000000" "KeepRelativeOffset" true)
  (return))

(fn GetStaticMesh
  (bind _array_element (Utilities|Array|ForEachLoopwithBreak (Actor|GetComponentsByClass (Components|GetOwner) "/Script/Engine.StaticMeshComponent") :!label _label)
    (:LoopBody
      (if (Utilities|Enum|Equal(Enum) (Utilities|GetObjectName _array_element) (Variables|Default|GetTypeOfCharacter))
        (Utilities|FlowControl|Sequence
          (:then_0
            (goto _label Break))
          (:then_1
            (bind _output_get (Variables|Default|SetCharacterStaticMesh _array_element))
            (CallFunction|ChangeDamageColor (Math|Vector|MakeVector 1.0 0.0 0.0))
            (CallFunction|ChangeSelectColor (Math|Vector|MakeVector 0.25 0.25 0.25))
            (return)))))))