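; Player component that picks and switches Jester sprite animations through the owner's BP_SpriteAnimation_Component.
; Tick flips the sprite mesh by X velocity direction and requests Idle or Moving.
; F plays an Override animation that blocks movement states until the sprite component reports its one-shot end.
; State requests only act on changes, setting animation type, speed and particle notify frames; Sprinting is defined but never requested.
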(event Custom|OverrideAnimation
  ;[1 1 1] Disables movement animations, calls a one shot type then when its finished reenables movement animations
  (Variables|Default|SetOverrideAnimationPlaying true)
  (CallFunction|RequestAnimationChange "Override"))

(event Custom|MovementAnimations
  ;[1 1 1] For the characters movement, get the actors velocity to determine animation speed/type
)

(event Custom|RequestAnimationChange
  (params (StateToChangeTo :type String))
  ;[1 1 1] Changes the animation if the requested state is different than the current
  (if (not (Utilities|Enum|Equal(Enum) StateToChangeTo (Variables|Default|GetCurrentState)))
    (bind _output_get (Variables|Default|SetCurrentState StateToChangeTo))
    (switch string _output_get
      (:Idle
        (Default|SetAnimationType (Variables|Default|GetPlayerSpriteComponentRef) "T_Jester" "NewEnumerator0" (Utilities|Array|MakeArray 0 0) (Utilities|Array|MakeArray "" "") 3333.0)
        (Development|PrintString "idle"))
      (:Moving
        (Default|SetAnimationType (Variables|Default|GetPlayerSpriteComponentRef) "T_Jester" "NewEnumerator0" (Utilities|Array|MakeArray 0 2 0) (Utilities|Array|MakeArray "" "SpawnFireParticles" "") 0.1)
        (Development|PrintString "moving"))
      (:Override
        (Default|SetAnimationType (Variables|Default|GetPlayerSpriteComponentRef) "T_Jester" "NewEnumerator1" (Utilities|Array|MakeArray 0 1 3 0) (Utilities|Array|MakeArray "" "SpawnFireParticles" "SpawnFireParticles" "") 0.4)
        (Development|PrintString "Hello"))
      (:Sprinting
        (Default|SetAnimationType (Variables|Default|GetPlayerSpriteComponentRef) "T_Jester" "NewEnumerator1" (Utilities|Array|MakeArray 0 1 3 0) (Utilities|Array|MakeArray "" "SpawnFireParticles" "SpawnFireParticles" "") 0.4)
        (Development|PrintString "Hello")))))

(event EventBeginPlay
  (bind _returnvalue (Components|GetOwner))
  (Variables|Default|SetPlayerActorRef _returnvalue)
  (Variables|Default|SetPlayerSpriteComponentRef (Actor|GetComponentbyClass _returnvalue "/Game/Characters/CharacterComponents/SpriteAnimation/BP_SpriteAnimation_Component.BP_SpriteAnimation_Component_C")))

(event EventTick
  (params (DeltaSeconds :type Float%20%28single-precision%29))
  (bind _playeractorref (Variables|Default|GetPlayerActorRef))
  (bind _playerspritecomponentref (Variables|Default|GetPlayerSpriteComponentRef))
  (bind _returnvalue (Transformation|GetVelocity _playeractorref))
  (bind _characterstaticmesh (Variables|/Game/Characters/CharacterComponents/SpriteAnimation/BP_SpriteAnimation_Component.BP_SpriteAnimation_Component_C|GetCharacterStaticMesh _playerspritecomponentref))
  (bind _returnvalue_2 (Math|Vector|Normalize (Math|Vector|MakeVector (.x _returnvalue) 0.0 0.0)))
  (if (Variables|/Game/Characters/CharacterComponents/SpriteAnimation/BP_SpriteAnimation_Component.BP_SpriteAnimation_Component_C|GetEndOfOneShotChangeAnimation (Variables|Default|GetPlayerSpriteComponentRef))
    (Variables|Default|SetOverrideAnimationPlaying false)
    (elif (Variables|Default|GetOverrideAnimationPlaying)
      (Variables|Default|SetOverrideAnimationPlaying true)
      (else
        (Variables|Default|SetOverrideAnimationPlaying false))))
  (if (> (.x _returnvalue_2) 0.0)
    (Transformation|SetRelativeRotation _characterstaticmesh "0.000000,0.000000,90.000000" false false)
    (elif (< (.x _returnvalue_2) 0.0)
      (Transformation|SetRelativeRotation _characterstaticmesh "0.000000,180.000000,90.000000" false false)))
  (bind _output_get (Variables|Default|SetVelocityNormalized (Math|Float|Absolute(Float) (.x _returnvalue_2))))
  (if (and (> _output_get 0.0) (== (Variables|Default|GetOverrideAnimationPlaying) false))
    (CallFunction|RequestAnimationChange "Moving")
    (if (> (.x _returnvalue) (Variables|Default|GetSprintSpeedThreshold))
      (Development|PrintString (Utilities|String|ToString(Vector) "0, 0, 0")))
    (elif (not (Variables|Default|GetOverrideAnimationPlaying))
      (CallFunction|RequestAnimationChange "Idle"))))

(event Input|KeyboardEvents|F
  (params (Key :type Key%20Structure :default "None"))
  (:Pressed
    (CallFunction|OverrideAnimation)))