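; Character component that owns the roster scroll UI, a list of NPC entries with name, portrait, tool, rank and proficiency.
; Creates the scroll widget on BeginPlay, and AddEntry and RemoveEntry feed BP_RosterScrollDataEntry objects into its list.
; SpaceBar opens or closes the scroll and toggles the mouse cursor.
; Debug keys add a randomized entry (T) and print the first displayed entry's name (S).
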(event Custom|AddEntry
  (params (Name :type Text) (Portrait :type Texture%202D%20Object%20Reference) (Tool :type Texture%202D%20Object%20Reference) (Rank :type Texture%202D%20Object%20Reference) (DefaultProficiency :type Float%20%28double-precision%29) (DefaultKills :type Integer))
  (bind _returnvalue (Game|ConstructObjectfromClass "/Game/Widgets/BP_RosterScrollDataEntry.BP_RosterScrollDataEntry_C"))
  (Default|Initialize _returnvalue Name Portrait Tool Rank DefaultProficiency DefaultKills)
  (Class|ListView|AddItem (Variables|/Game/Widgets/WBP_RosterScroll.WBP_RosterScroll_C|GetRosterScrollList (Variables|Default|GetRosterScrollWidget)) _returnvalue))

(event Custom|RemoveEntry
  (params (Item :type Object%20Object%20Reference))
  ;[1 1 1] Npcs will pass over their own roster scroll data entry here, it will also be destroyed by the list
  (Class|ListView|RemoveItem (Variables|/Game/Widgets/WBP_RosterScroll.WBP_RosterScroll_C|GetRosterScrollList (Variables|Default|GetRosterScrollWidget)) Item))

(event EventBeginPlay
  (bind _returnvalue (UserInterface|CreateWidget "/Game/Widgets/WBP_RosterScroll.WBP_RosterScroll_C"))
  (Variables|Default|SetRosterScrollWidget _returnvalue)
  (UserInterface|Viewport|AddtoViewport _returnvalue 0)
  (Class|UserWidget|SetAnchorsinViewport _returnvalue (Utilities|Struct|MakeAnchors "(X=0.000000,Y=0.500000)" "(X=0.000000,Y=0.000000)")))

(event Input|KeyboardEvents|T
  (params (Key :type Key%20Structure :default "None"))
  (:Pressed
    (bind _returnvalue (Game|ConstructObjectfromClass "/Game/Widgets/BP_RosterScrollDataEntry.BP_RosterScrollDataEntry_C"))
    (Default|Initialize _returnvalue (Utilities|Select :Index (Math|Random|RandomIntegerinRange 0 2) :Option%200 "Dave" :Option%201 "Joeee" :Option%202 "Peta") (Utilities|Select :Index (Math|Random|RandomIntegerinRange 0 2) :Option%200 "/Engine/EngineResources/AICON-Red.AICON-Red" :Option%201 "/Engine/EngineResources/AICON-Green.AICON-Green" :Option%202 "/Engine/Tutorial/Mobile/TutorialAssets/android_Icon.android_Icon") (Utilities|Select :Index (Math|Random|RandomIntegerinRange 0 2) :Option%200 "/Engine/EngineResources/AICON-Red.AICON-Red" :Option%201 "/Engine/EngineResources/AICON-Green.AICON-Green" :Option%202 "/Engine/Tutorial/Mobile/TutorialAssets/android_Icon.android_Icon") (Utilities|Select :Index (Math|Random|RandomIntegerinRange 0 2) :Option%200 "/Engine/EngineResources/AICON-Red.AICON-Red" :Option%201 "/Engine/EngineResources/AICON-Green.AICON-Green" :Option%202 "/Engine/Tutorial/Mobile/TutorialAssets/android_Icon.android_Icon") (Math|Random|RandomFloatinRange -1.0 1.0))
    (Class|ListView|AddItem (Variables|/Game/Widgets/WBP_RosterScroll.WBP_RosterScroll_C|GetRosterScrollList (Variables|Default|GetRosterScrollWidget)) _returnvalue)))

(event Input|KeyboardEvents|S
  (params (Key :type Key%20Structure :default "None"))
  (:Pressed
    (bind _aswbp_roster_scroll_entry (Utilities|Casting|CastToWBP_RosterScrollEntry (Utilities|Array|Get(acopy) (Class|ListViewBase|GetDisplayedEntryWidgets (Variables|/Game/Widgets/WBP_RosterScroll.WBP_RosterScroll_C|GetRosterScrollList (Variables|Default|GetRosterScrollWidget))))))
    (Development|PrintString (Utilities|String|ToString(Text) (Variables|/Script/UMG.EditableText|GetText (Variables|/Game/Widgets/WBP_RosterScrollEntry.WBP_RosterScrollEntry_C|GetNameTag _aswbp_roster_scroll_entry))))))

(event Input|KeyboardEvents|SpaceBar
  (params (Key :type Key%20Structure :default "None"))
  (bind _returnvalue (Game|GetPlayerController 0))
  (bind _rosterscrollwidget (Variables|Default|GetRosterScrollWidget))
  (:Pressed
    (if (Variables|Default|GetScrollOpen)
      (Variables|Default|SetScrollOpen false)
      (Variables|/Script/Engine.PlayerController|SetbShowMouseCursor _returnvalue false)
      (Default|CloseScroll _rosterscrollwidget)
      (else
        (Variables|Default|SetScrollOpen true)
        (Variables|/Script/Engine.PlayerController|SetCurrentMouseCursor _returnvalue "EyeDropper")
        (Variables|/Script/Engine.PlayerController|SetbShowMouseCursor _returnvalue true)
        (Default|OpenScroll _rosterscrollwidget)))))