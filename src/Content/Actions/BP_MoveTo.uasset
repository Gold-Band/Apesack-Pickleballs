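; BP_MoveTo is an action that moves a pawn toward a target actor along the world X axis.
; Init caches the owning actor as a Pawn and stores the target.
; Each run applies movement input along the pawn's forward vector, signed by the target's relative X position.
; It returns Success with the target once X distance drops below StopDist, InProgress until then, or Failed if either reference is invalid.
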(event EventRecieveInit
  (params (OwningActorRef :type Actor%20Object%20Reference) (TargetRef :type Actor%20Object%20Reference))
  (bind _aspawn (Utilities|Casting|CastToPawn OwningActorRef))
  (Variables|Default|SetAs%20Pawn _aspawn)
  (if (Utilities|IsValid TargetRef)
    (Variables|Default|SetTarget%20Ref TargetRef)))

(fn RecieveRun
  (bind _target_ref (Variables|Default|GetTarget%20Ref))
  (bind _as_pawn (Variables|Default|GetAs%20Pawn))
  (bind _returnvalue (Transformation|GetActorLocation _target_ref))
  (bind _returnvalue_2 (Transformation|GetActorLocation _as_pawn))
  (bind _returnvalue_3 (- (.x _returnvalue) (.x _returnvalue_2)))
  (if (and (Utilities|IsValid (Variables|Default|GetTarget%20Ref)) (Utilities|IsValid (Variables|Default|GetAs%20Pawn)))
    (Pawn|Input|AddMovementInput (Variables|Default|GetAs%20Pawn) (Transformation|GetActorForwardVector (Variables|Default|GetAs%20Pawn)) (Math|Float|SelectFloat 1.0 -1.0 (> _returnvalue_3 0.0)) false)
    (if (< (Math|Float|Absolute(Float) _returnvalue_3) (Variables|Default|GetStopDist))
      (Variables|Default|SetReturnedTarget (Variables|Default|GetTarget%20Ref))
      (return "Success")
      (else
        (return "InProgress")))
    (else
      (return "Failed"))))