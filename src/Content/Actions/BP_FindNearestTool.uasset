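; BP_FindNearestTool is an action that finds the closest actor carrying a given tag, relative to its owning actor.
; When run, it gathers the actors matching FindTag and picks the nearest to the owner's location as ReturnedTarget.
; It returns Success if that target is valid, and Failed if either the owner or the target is invalid.
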(fn RecieveRun
  (Utilities|IsValid (Variables|Default|GetOwningActor)
    (:Is%20Valid
      (bind _returnvalue (Class|FindObjectTask|FindActorswithTag (Variables|Default|GetFindTag)))
      (bind _output_get (Variables|Default|SetReturnedTarget (.ReturnValue (Actor|FindNearestActor (Transformation|GetActorLocation (Variables|Default|GetOwningActor)) _returnvalue))))
      (Utilities|IsValid _output_get
        (:Is%20Valid
          (return "Success"))
        (:Is%20Not%20Valid
          (return "Failed"))))
    (:Is%20Not%20Valid
      (return "Failed"))))