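; Player character Blueprint that handles coin pickup and coin-paid interaction with overlapped objects.
; Box collider overlaps feed the Interactor component, and begin overlaps also go to coin handling.
; A coin either starts spinning and interpolating to the player or, once flagged to count, increments coins, hides itself and spawns a burst effect.
; The Interact input spends the Interactor's requested coins and interacts only if that succeeds.
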(event OnComponentBeginOverlap(BoxCollider)
  (params (OverlappedComponent :type Primitive%20Component%20Object%20Reference) (OtherActor :type Actor%20Object%20Reference) (OtherComp :type Primitive%20Component%20Object%20Reference) (OtherBodyIndex :type Integer) (bFromSweep :type Boolean) (SweepResult :type Hit%20Result%20Structure%20%28by%20ref%29))
  (Class|Interactor|BeginInteractOverlap (Variables|Default|GetInteractor) OtherActor)
  (CallFunction|CoinInterpolationorCollision OtherActor))

(event OnComponentEndOverlap(BoxCollider)
  (params (OverlappedComponent :type Primitive%20Component%20Object%20Reference) (OtherActor :type Actor%20Object%20Reference) (OtherComp :type Primitive%20Component%20Object%20Reference) (OtherBodyIndex :type Integer))
  (Class|Interactor|EndInteractOverlap (Variables|Default|GetInteractor) OtherActor))

(event Input|EnhancedActionEvents|EnhancedInputActionIA_Interact
  (params (ActionValue :type Boolean) (ElapsedSeconds :type Float%20%28double-precision%29) (TriggeredSeconds :type Float%20%28double-precision%29) (InputAction :type Input%20Action%20Object%20Reference :default "/Game/Input/IA_Interact.IA_Interact"))
  (bind _interactor (Variables|Default|GetInteractor))
  (:Started
    (bind _returnvalue (Class|Interactor|RequestedCoins _interactor))
    (bind _returnvalue_2 (Class|PlayerCharacter|SpendCoins _returnvalue))
    (if _returnvalue_2
      (Class|Interactor|Interact _interactor))))

(event EventBeginPlay)

(fn ConstructionScript)

(fn CoinInterpolationorCollision
  (params (Object :type Object%20Object%20Reference))
  (bind _asbp_coin (Utilities|Casting|CastToBP_Coin Object))
  (if (Variables|/Game/Blueprints/Coin/BP_Coin.BP_Coin_C|GetShouldIncrementCoinCount _asbp_coin)
    (if (not (Variables|/Game/Blueprints/Coin/BP_Coin.BP_Coin_C|GetDisabledVisuals _asbp_coin))
      (Class|PlayerCharacter|IncrementCoins)
      (Default|DisableParticleSystemandCoinMesh _asbp_coin)
      (Effects|SpawnEmitterAttached "/Game/Effects/PS_CoinGainedBurst.PS_CoinGainedBurst" (Variables|Default|GetBox%20Collider) "None")
      (return))
    (else
      (Default|InterpolatetoPlayer _asbp_coin self)
      (Variables|/Game/Blueprints/Coin/BP_Coin.BP_Coin_C|SetShouldStartSpinning _asbp_coin true))))