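; Enemy pawn that homes in on the player character, BP_Dude, in a straight line.
; BeginPlay caches the first BP_Dude found in the level.
; Each Tick offsets the pawn along the normalized direction to that actor, scaled by EnemySpeed.
; Movement has no sweep, pathfinding or delta-time scaling, so it ignores collision along the way and varies with frame rate.
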(event EventBeginPlay
  ;[1 1 1] Get Player Reference
  (bind _returnvalue (Actor|GetActorOfClass "/Game/BP_Dude.BP_Dude_C"))
  (Variables|Default|SetBP_DudeRef _returnvalue))

(event EventTick
  (params (DeltaSeconds :type Float%20%28single-precision%29))
  ;[1 1 1 1 69] Move Enemy Towards Player
  (Transformation|AddActorWorldOffset (* (* (Math|Vector|Normalize (- (Transformation|GetActorLocation) (Transformation|GetActorLocation (Variables|Default|GetBP_DudeRef)))) (Math|Conversions|ToVector(Float) (Variables|Default|GetEnemySpeed))) "-1.000000,-1.000000,-1.000000")))

(fn ConstructionScript)