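; Camera follow Blueprint that moves the level's camera along the X axis to track the player's Jester component.
; On BeginPlay it caches the first CameraActor and BP_PlayerCharacterController found in the level.
; Each Tick it lerps a stored X toward Jester's world X with a fixed alpha, so smoothing depends on frame rate.
; The camera takes that X plus an offset, while Y and Z come solely from the offset.
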(event EventBeginPlay
  (bind _returnvalue (Actor|GetActorOfClass "/Script/Engine.CameraActor"))
  (Variables|Default|SetMainCamera _returnvalue)
  (bind _returnvalue_2 (Actor|GetActorOfClass "/Game/Blueprints/Player/BP_PlayerCharacterController.BP_PlayerCharacterController_C"))
  (Variables|Default|SetPlayerControllerRef _returnvalue_2))

(event EventTick
  (params (DeltaSeconds :type Float%20%28single-precision%29))
  (bind _offset (Variables|Default|GetOffset))
  (bind (_x _y _z) (Math|Vector|BreakVector _offset))
  (bind _output_get (Variables|Default|SetCurrentCameraXLocation (Math|Float|Lerp (Variables|Default|GetCurrentCameraXLocation) (* (.x (Transformation|GetWorldLocation (Variables|/Game/Blueprints/Player/BP_PlayerCharacterController.BP_PlayerCharacterController_C|GetJester (Variables|Default|GetPlayerControllerRef)))) 1.0) 0.3)))
  (Transformation|SetActorLocation (Variables|Default|GetMainCamera) (Math|Vector|MakeVector (+ _output_get _x) _y _z) false false))

(fn ConstructionScript)